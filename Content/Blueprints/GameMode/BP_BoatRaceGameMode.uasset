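; BP_BoatRaceGameMode is the boat race game mode, handling the start countdown.
; On BeginPlay it caches BP_BoatGameInstance, then shows WBP_RaceStartTimer under UI-only input.
; Game input returns one second before the countdown value elapses, and the widget is removed a second later.
; Unconnected logic would spawn and possess the selected boat at a PlayerStart and apply the chosen character mesh, but it never runs.
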(event `self.ReceiveBeginPlay`
  (`|ExecutionSequence`
    (:`then_0`
      (bind _asbp_boat_game_instance (cast `/Game/Blueprints/GameInstance/BP_BoatGameInstance` (`GameplayStatics.GetGameInstance`)))
      (set `self.BoatGameInstacne` _asbp_boat_game_instance))
    (:`then_2`
      (`WidgetBlueprintLibrary.SetInputMode_UIOnlyEx` (`GameplayStatics.GetPlayerController` 0) null)
      (`self.HandlingRaceWidget`)
      (`KismetSystemLibrary.Delay` (- (`self.SetCountDownValue`) 1.0))
      (`WidgetBlueprintLibrary.SetInputMode_GameOnly` (`GameplayStatics.GetPlayerController` 0))
      (`KismetSystemLibrary.Delay` 1.0)
      (`Widget.RemoveFromParent` (`self.RaceStartWidget`)))))

(fn `FindBoatPlayerStart`
  (returns (BoatPlayerStart :type "Transform Structure (by ref)"))
  (bind _returnvalue (`GameplayStatics.GetActorOfClass` "/Script/Engine.PlayerStart"))
  (return (`self.GetTransform` _returnvalue)))

(fn `HandlingRaceWidget`
  (bind _returnvalue (`|CreateWidget` "/Game/Blueprints/UI/GameEvents/WBP_RaceStartTimer.WBP_RaceStartTimer_C"))
  (bind _output_get (set `self.RaceStartWidget` _returnvalue))
  (`UserWidget.AddToViewport` _output_get 0)
  (`/Game/Blueprints/UI/GameEvents/WBP_RaceStartTimer.SetCountDownValue` (`self.RaceStartWidget`) (`self.SetCountDownValue`))
  (`/Game/Blueprints/UI/GameEvents/WBP_RaceStartTimer.SetRaceTimer` (`self.RaceStartWidget`) 0.0))

(fn `UserConstructionScript`)