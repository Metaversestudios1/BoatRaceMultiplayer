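; Base boat Blueprint that drives wave interaction by acting as a dynamic force in the BP_FluidSim_01 fluid simulation.
; On BeginPlay it finds the sim actor and registers its FluidSimulation component with a configurable radius, strength and boat-specific force material.
; Each Tick it checks IsInAir, re-registering with zero force when airborne and restoring the force otherwise, using ValidFluidSim to avoid repeat registration.
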(event `self.ReceiveBeginPlay`
  (`self.WaveSimulation`))

(event `self.ReceiveTick`
  (params (DeltaSeconds :type "Float (single-precision)"))
  (`self.HandlingFluidSimulation`))

(fn `HandlingFluidSimulation`
  (bind _fluidsimulation (`self.FluidSimulation`))
  (if (`self.bIsInAir`)
    (if (`self.bValidFluidSim`)
      (bind _fluidsim (`self.FluidSim`)
        (:`then`
          (`/Water/FluidSimulation/Blueprints/BP_FluidSim_01.Register Dynamic Force` _fluidsim (make `/Water/FluidSimulation/Blueprints/Structs/FluidForceDynamic` "NewEnumerator0" 0.0 0.0 _fluidsimulation) _fluidsimulation 0.0)
          (set `self.bValidFluidSim` false))
        (:`else`)))
    (elif (not (`self.bValidFluidSim`))
      (`self.RegisterFluidDynamicForce`))))

(fn `RegisterFluidDynamicForce`
  (bind _fluidsimulation (`self.FluidSimulation`))
  (bind _fluidsim (`self.FluidSim`)
    (:`then`
      (`/Water/FluidSimulation/Blueprints/BP_FluidSim_01.Register Dynamic Force` _fluidsim (make `/Water/FluidSimulation/Blueprints/Structs/FluidForceDynamic` "NewEnumerator0" (`self.FluidForceRadius`) (`self.FluidForceStrenght`) _fluidsimulation "/Water/FluidSimulation/Materials/Forces/M_Fluid_Sim_Force_Boat_Component.M_Fluid_Sim_Force_Boat_Component" (make `/Water/FluidSimulation/Blueprints/Structs/FluidForceSocketInfo` (`|MakeMap` "None" :!type "Name" :!valuetype "Name"))) _fluidsimulation 0.0)
      (set `self.bValidFluidSim` true))
    (:`else`)))

(fn `UserConstructionScript`)

(fn `WaveSimulation`
  (bind _returnvalue (`GameplayStatics.GetActorOfClass` "/Water/FluidSimulation/Blueprints/BP_FluidSim_01.BP_FluidSim_01_C"))
  (set `self.FluidSim` _returnvalue)
  (`self.RegisterFluidDynamicForce`))