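; BP_ChangeCharacter swaps the boat character shown for character selection and records the choice in the game instance.
; On BeginPlay it stores the length of the BoatCharacters array as MaxCharacters and caches the BP_BoatGameInstance.
; SetBoatCharacter applies the indexed skeletal mesh to the BoatCharacter component and, if the game instance is valid, saves that mesh as CharacterSelected.
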(event `self.ReceiveBeginPlay`
  (set `self.MaxCharacters` (`KismetArrayLibrary.Array_Length` (`self.BoatCharacters`)))
  (bind _asbp_boat_game_instance (cast `/Game/Blueprints/GameInstance/BP_BoatGameInstance` (`GameplayStatics.GetGameInstance`)))
  (set `self.BoatGameInstance` _asbp_boat_game_instance))

(fn `SetBoatCharacter`
  (params (Index :type Integer))
  (bind _output (`|GetArrayItem` (`self.BoatCharacters`) Index))
  (`SkeletalMeshComponent.SetSkeletalMeshAsset` (`self.BoatCharacter`) _output)
  (bind _boatgameinstance (`self.BoatGameInstance`)
    (:`then`
      (set `/Game/Blueprints/GameInstance/BP_BoatGameInstance.CharacterSelected` _output _boatgameinstance))
    (:`else`)))

(fn `UserConstructionScript`)