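; Selection actor that previews boat and character dress choices and records them in BP_BoatGameInstance.
; BeginPlay caches the game instance and derives boat and dress limits from their arrays, subtracting one only for dresses.
; SetBoatMesh shows the mesh at the passed Index but saves the class at BoatIndex.
; SetCharacterDress saves the material at CharacterDressIndex and applies it to one character material slot.
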(event `self.ReceiveBeginPlay`
  (bind _asbp_boat_game_instance (cast `/Game/Blueprints/GameInstance/BP_BoatGameInstance` (`GameplayStatics.GetGameInstance`)))
  (set `self.BoatGameInstance` _asbp_boat_game_instance)
  (set `self.MaxBoatCount` (`KismetArrayLibrary.Array_Length` (`self.Boats`)))
  (set `self.MaxCharacterDressCount` (- (`KismetArrayLibrary.Array_Length` (`self.CharacterDressMaterial`)) 1)))

(fn `SetBoatMesh`
  (params (Index :type Integer))
  (`StaticMeshComponent.SetStaticMesh` (`self.Boat`) (`|GetArrayItem` (`self.Boats`) Index))
  (bind _boatgameinstance (`self.BoatGameInstance`)
    (:`then`
      (set `/Game/Blueprints/GameInstance/BP_BoatGameInstance.BoatSelected` (`|GetArrayItem` (`self.BoatClass`) (`self.BoatIndex`)) _boatgameinstance))
    (:`else`)))

(fn `SetCharacterDress`
  (bind _boatgameinstance (`self.BoatGameInstance`)
    (:`then`
      (bind _output_get (set `/Game/Blueprints/GameInstance/BP_BoatGameInstance.CharacterDressSelected` (`|GetArrayItem` (`self.CharacterDressMaterial`) (`self.CharacterDressIndex`)) _boatgameinstance))
      (`PrimitiveComponent.SetMaterial` (`self.BoatCharcter`) 16 _output_get))
    (:`else`)))

(fn `UserConstructionScript`)