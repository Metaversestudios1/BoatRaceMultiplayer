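; BP_ChangeBoat is a boat selection Blueprint that swaps the displayed boat mesh and records the chosen boat class.
; BeginPlay caches the boat count and the BP_BoatGameInstance.
; SetBoatMesh applies a mesh from the Boats array to the Boat component and, if the game instance is valid, writes the BoatClass entry to its BoatSelected.
; The mesh lookup uses the Index parameter, while the class lookup uses the BoatIndex variable.
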(event `self.ReceiveBeginPlay`
  (set `self.MaxBoats` (`KismetArrayLibrary.Array_Length` (`self.Boats`)))
  (bind _asbp_boat_game_instance (cast `/Game/Blueprints/GameInstance/BP_BoatGameInstance` (`GameplayStatics.GetGameInstance`)))
  (set `self.BoatGameInstance` _asbp_boat_game_instance))

(fn `SetBoatMesh`
  (params (Index :type Integer))
  (`StaticMeshComponent.SetStaticMesh` (`self.Boat`) (`|GetArrayItem` (`self.Boats`) Index))
  (bind _boatgameinstance (`self.BoatGameInstance`)
    (:`then`
      (set `/Game/Blueprints/GameInstance/BP_BoatGameInstance.BoatSelected` (`|GetArrayItem` (`self.BoatClass`) (`self.BoatIndex`)) _boatgameinstance))
    (:`else`)))

(fn `UserConstructionScript`)